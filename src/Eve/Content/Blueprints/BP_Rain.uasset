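; BP_Rain is a character Blueprint carrying a foot IK system for ABP_Mannequin_noroot, currently inactive because Tick is empty and the IK calls are unwired.
; BeginPlay caches the AnimInstance, and construction stores the scaled capsule half-height.
; IKUpdate line-traces below each foot socket, then interpolates foot rotation, effector offsets, hip drop and capsule height.
; IKResetVars eases those values back, while jump and climb-idle hooks are empty stubs.
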(event EventTick
  (params (DeltaSeconds :type Float%20%28single-precision%29)))

(event EventBeginPlay
  (bind _asabp_mannequin_noroot (Utilities|Casting|CastToABP_Mannequin_noroot (Components|SkeletalMesh|GetAnimInstance (Variables|Character|GetMesh))))
  (Variables|Default|SetAnimInstance _asabp_mannequin_noroot))

(event EventOnJumpStart)

(fn ConstructionScript
  ;[1 1 1] Ensuring that IK works with scale
  (Variables|Default|SetIKCapsuleHalfHeight (Components|Capsule|GetScaledCapsuleHalfHeight (Variables|Default|GetCapsuleComponent))))

(fn IKFootTrace
  (params (TraceDistance :type Float%20%28single-precision%29) (SocketName :type Name))
  (bind _returnvalue (Transformation|GetActorLocation))
  (bind _mesh (Variables|Character|GetMesh))
  (bind _returnvalue_2 (Transformation|GetSocketLocation _mesh SocketName))
  (bind _outhit (Collision|LineTraceByChannel (Math|Vector|MakeVector (.x _returnvalue_2) (.y _returnvalue_2) (.z _returnvalue)) (Math|Vector|MakeVector (.x _returnvalue_2) (.y _returnvalue_2) (- (- (.z _returnvalue) (Variables|Default|GetIKCapsuleHalfHeight)) TraceDistance)) "TraceTypeQuery1" true 0 "ForOneFrame" true "(R=0.000000,G=0.000000,B=0.000000,A=0.000000)"))
  (return (Math|Float|SelectFloat (+ (Variables|Default|GetIKAdjustOffset) (- (Math|Vector|VectorLength (- (.location _outhit) (.traceend _outhit))) TraceDistance)) 0.0 (.bblockinghit _outhit)) (.impactnormal _outhit)))

(fn IKNormaltoRotator
  (params (Normal :type Vector))
  (return (Math|Rotator|MakeRotator (Class|KismetMathLibrary|DegAtan2 (.y Normal) (.z Normal)) (* (Class|KismetMathLibrary|DegAtan2 (.x Normal) (.z Normal)) -1.0) 0.0)))

(fn IKUpdateFootOffset
  (params (TargetValue :type Float%20%28single-precision%29) (Effector :type Float%20%28single-precision%29%20%28by%20ref%29) (InterpSpeed :type Float%20%28single-precision%29))
  (|SetBy-RefVar Effector (Math|Interpolation|FInterpTo Effector TargetValue (Utilities|Time|GetWorldDeltaSeconds) InterpSpeed)))

(fn IKUpdateFootRotation
  (params (TargetValue :type Rotator) (Rotation :type Rotator%20%28by%20ref%29) (InterpSpeed :type Float%20%28single-precision%29))
  (|SetBy-RefVar Rotation (Math|Interpolation|RInterpTo Rotation TargetValue (Utilities|Time|GetWorldDeltaSeconds) InterpSpeed)))

(fn IKUpdateCapsuleHalfHeight
  (params (HipsShift :type Float%20%28single-precision%29) (ResetToDefault :type Boolean))
  (bind _capsulecomponent (Variables|Default|GetCapsuleComponent))
  (bind _ikcapsulehalfheight (Variables|Default|GetIKCapsuleHalfHeight))
  (Components|Capsule|SetCapsuleHalfHeight _capsulecomponent (Math|Interpolation|FInterpTo (Components|Capsule|GetScaledCapsuleHalfHeight _capsulecomponent) (Math|Float|SelectFloat _ikcapsulehalfheight (- _ikcapsulehalfheight (/ (Math|Float|Absolute(Float) HipsShift) 2.0)) ResetToDefault) (Utilities|Time|GetWorldDeltaSeconds) (Variables|Default|GetIKHipsInterpSpeed)) true))

(fn IKResetVars
  (bind _animinstance (Variables|Default|GetAnimInstance))
  (bind _ikfeetinterpspeed (Variables|Default|GetIKFeetInterpSpeed))
  (bind _animinstance_2 (Variables|Default|GetAnimInstance))
  (bind _ikfeetinterpspeed_2 (Variables|Default|GetIKFeetInterpSpeed))
  (Utilities|FlowControl|Sequence
    (:then_0
      (CallFunction|IKUpdateFootOffset 0.0 (Variables|/Game/Meshes/UE4_Mannequin_with_Root/ABP_Mannequin_noroot.ABP_Mannequin_noroot_C|GetRightFootEffectorLocation _animinstance) _ikfeetinterpspeed)
      (CallFunction|IKUpdateFootOffset 0.0 (Variables|/Game/Meshes/UE4_Mannequin_with_Root/ABP_Mannequin_noroot.ABP_Mannequin_noroot_C|GetLeftFootEffectorLocation _animinstance) _ikfeetinterpspeed))
    (:then_1
      (CallFunction|IKUpdateFootRotation "0, 0, 0" (Variables|/Game/Meshes/UE4_Mannequin_with_Root/ABP_Mannequin_noroot.ABP_Mannequin_noroot_C|GetRightFootRotation _animinstance_2) _ikfeetinterpspeed_2)
      (CallFunction|IKUpdateFootRotation "0, 0, 0" (Variables|/Game/Meshes/UE4_Mannequin_with_Root/ABP_Mannequin_noroot.ABP_Mannequin_noroot_C|GetLeftFootRotation _animinstance_2) _ikfeetinterpspeed_2))
    (:then_2
      (CallFunction|IKUpdateFootOffset 0.0 (Variables|/Game/Meshes/UE4_Mannequin_with_Root/ABP_Mannequin_noroot.ABP_Mannequin_noroot_C|GetHipsOffset (Variables|Default|GetAnimInstance)) (Variables|Default|GetIKHipsInterpSpeed))
      (CallFunction|IKUpdateCapsuleHalfHeight 0.0 false))))

(fn IKUpdate
  (bind _ikoffsetleftfoot (Variables|Default|GetIKOffsetLeftFoot))
  (bind _ikoffsetrightfoot (Variables|Default|GetIKOffsetRightFoot))
  (bind _returnvalue (Math|Float|Min(Float) _ikoffsetleftfoot _ikoffsetrightfoot))
  (bind _returnvalue_2 (< _returnvalue 0.0))
  (bind _returnvalue_3 (Math|Float|SelectFloat _returnvalue 0.0 _returnvalue_2))
  (Utilities|FlowControl|Sequence
    (:then_0
      (bind (_ikoffset _impactnormal) (CallFunction|IKFootTrace (Variables|Default|GetFootIKTraceDistance) (Variables|Default|GetIKLeftSocket)))
      (CallFunction|IKUpdateFootRotation (CallFunction|IKNormaltoRotator _impactnormal) (Variables|/Game/Meshes/UE4_Mannequin_with_Root/ABP_Mannequin_noroot.ABP_Mannequin_noroot_C|GetLeftFootRotation (Variables|Default|GetAnimInstance)) (Variables|Default|GetIKFeetInterpSpeed)))
    (:then_1
      (bind (_ikoffset_2 _impactnormal_2) (CallFunction|IKFootTrace (Variables|Default|GetFootIKTraceDistance) (Variables|Default|GetIKRightSocket)))
      (CallFunction|IKUpdateFootRotation (CallFunction|IKNormaltoRotator _impactnormal_2) (Variables|/Game/Meshes/UE4_Mannequin_with_Root/ABP_Mannequin_noroot.ABP_Mannequin_noroot_C|GetRightFootRotation (Variables|Default|GetAnimInstance)) (Variables|Default|GetIKFeetInterpSpeed)))
    (:then_2
      (CallFunction|IKUpdateFootOffset _returnvalue_3 (Variables|/Game/Meshes/UE4_Mannequin_with_Root/ABP_Mannequin_noroot.ABP_Mannequin_noroot_C|GetHipsOffset (Variables|Default|GetAnimInstance)) (Variables|Default|GetIKHipsInterpSpeed))
      (CallFunction|IKUpdateCapsuleHalfHeight _returnvalue_3 false))
    (:then_3
      (CallFunction|IKUpdateFootOffset (- _ikoffset _returnvalue_3) (Variables|/Game/Meshes/UE4_Mannequin_with_Root/ABP_Mannequin_noroot.ABP_Mannequin_noroot_C|GetLeftFootEffectorLocation (Variables|Default|GetAnimInstance)) (Variables|Default|GetIKFeetInterpSpeed))
      (CallFunction|IKUpdateFootOffset (- _ikoffset_2 _returnvalue_3) (Variables|/Game/Meshes/UE4_Mannequin_with_Root/ABP_Mannequin_noroot.ABP_Mannequin_noroot_C|GetRightFootEffectorLocation (Variables|Default|GetAnimInstance)) (Variables|Default|GetIKFeetInterpSpeed)))
    (:then_4
      (if (and (Math|Float|NearlyEqual(Float) (Variables|/Game/Meshes/UE4_Mannequin_with_Root/ABP_Mannequin_noroot.ABP_Mannequin_noroot_C|GetLeftFootEffectorLocation (Variables|Default|GetAnimInstance)) (- (Variables|Default|GetIKOffsetLeftFoot) _returnvalue_3) 1.0) (Math|Float|NearlyEqual(Float) (Variables|/Game/Meshes/UE4_Mannequin_with_Root/ABP_Mannequin_noroot.ABP_Mannequin_noroot_C|GetRightFootEffectorLocation (Variables|Default|GetAnimInstance)) (- (Variables|Default|GetIKOffsetRightFoot) _returnvalue_3) 1.0))
        _))))

(fn AdjustBodyOffsetforClimbIdle)