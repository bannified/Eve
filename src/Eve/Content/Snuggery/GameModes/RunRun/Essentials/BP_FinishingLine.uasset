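; BP_FinishingLine is the finish line actor for the RunRun game mode, though it does not yet act on a finish.
; Its zone's begin-overlap event prints a debug message naming the overlapping component and actor, then casts the actor to BP_RunRunCharacter with nothing after it.
; The construction script is empty; disconnected nodes hold unused logic to scale the line visual by length and tint it through a dynamic material.
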(event EventOnComponentBeginOverlapZone
  (params (OverlappedComponent :type Primitive%20Component%20Object%20Reference) (OtherActor :type Actor%20Object%20Reference) (OtherComp :type Primitive%20Component%20Object%20Reference))
  (Development|PrintString (Utilities|String|Append (Utilities|GetDisplayName OtherComp) " is overlapping " " at component: " (Utilities|GetDisplayName OtherActor)) true true "(R=0.000000,G=0.660000,B=1.000000,A=1.000000)" 5e+01)
  (Utilities|Casting|CastToBP_RunRunCharacter OtherActor))

(fn ConstructionScript)