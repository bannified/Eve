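; Player controller for Snuggery that routes key presses to widgets owned by BP_SnuggeryHUD.
; Enter sets focus on the chat box inside the player UI widget.
; The Info input action toggles the character selection view, switching to Game and UI input mode when showing it.
; Hiding the view leaves the input mode unchanged.
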(event EventBeginPlay)

(event Input|ActionEvents|InputActionInfo
  (params (Key :type Key%20Structure :default "None"))
  (:Pressed
    (bind _asbp_snuggery_hud (Utilities|Casting|CastToBP_SnuggeryHUD (HUD|GetHUD)))
    (switch Utilities|FlowControl|Switch|SwitchonESlateVisibility (Widget|GetVisibility (Variables|/Game/Snuggery/Widgets/BP_SnuggeryHUD.BP_SnuggeryHUD_C|GetWBP_CharacterSelectionView _asbp_snuggery_hud))
      (:Visible
        (Widget|SetVisibility (Variables|/Game/Snuggery/Widgets/BP_SnuggeryHUD.BP_SnuggeryHUD_C|GetWBP_CharacterSelectionView _asbp_snuggery_hud) "Hidden"))
      (:Collapsed
        (Widget|SetVisibility (Variables|/Game/Snuggery/Widgets/BP_SnuggeryHUD.BP_SnuggeryHUD_C|GetWBP_CharacterSelectionView _asbp_snuggery_hud) "Visible" :!label _label)
        (Input|SetInputModeGameandUI (Game|GetPlayerController 0) 0 "DoNotLock" false))
      (:Hidden
        (goto _label))
      (:HitTestInvisible
        (goto _label))
      (:SelfHitTestInvisible
        (goto _label)))))

(event Input|KeyboardEvents|Enter
  (params (Key :type Key%20Structure :default "None"))
  (:Pressed
    (bind _asbp_snuggery_hud (Utilities|Casting|CastToBP_SnuggeryHUD (HUD|GetHUD)))
    (Default|SetChatBoxFocus (Variables|/Game/Snuggery/Widgets/WBP_SnuggeryPlayerUI.WBP_SnuggeryPlayerUI_C|GetWBP_Chatbox (Variables|/Game/Snuggery/Widgets/BP_SnuggeryHUD.BP_SnuggeryHUD_C|GetWBP_PlayerUI _asbp_snuggery_hud)))))

(fn ConstructionScript)